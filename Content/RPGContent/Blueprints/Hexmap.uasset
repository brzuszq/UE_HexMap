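; Hexmap actor that creates, saves and loads a hexagon-shaped map of Tile actors.
; CreateHexMap spawns default tiles within a diameter-squared grid, padding TileArray outside the hexagon so coordinates convert directly to indices for six-neighbour lookups.
; SaveMap writes tile properties, radius, player tile and seed to SaveBP; LoadMap clears tiles, restores these and respawns through SpawnMap.
; CreateMap, Reload and TranslocateMap contain only disconnected logic.
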(event EventBeginPlay)

(event Collision|EventActorBeginOverlap
  (params (OtherActor :type Actor%20Object%20Reference)))

(event EventTick
  (params (DeltaSeconds :type Float%20%28single-precision%29)))

(fn ConstructionScript
  (Variables|Default|SetHexDiameter (- (* (Variables|MapCreation|GetHexmapRadius) 2) 1))
  (Development|PrintString "Hexmap Contruction!!!" true true "(R=1.000000,G=0.017204,B=0.000000,A=1.000000)" 2e+01))

(fn CreateMap)

(fn DestroyMap
  (bind _tilearray (Variables|Default|GetTileArray))
  (for _array_element _tilearray
    (Actor|DestroyActor _array_element))
  (Utilities|Array|Clear _tilearray))

(fn SaveMap
  (bind _returnvalue (SaveGame|CreateSaveGameObject "/Game/RPGContent/Blueprints/SaveBP.SaveBP_C"))
  (Variables|Default|SetSaveRef _returnvalue)
  (Utilities|FlowControl|Sequence
    (:then_0
      ;[1 1 1] Save Data
      (for _array_element (Variables|Default|GetTileArray)
        (Utilities|Array|Add (LocalVariables|GetTempArray) (Variables|/Game/RPGContent/Blueprints/Tile.Tile_C|GetTileProperties _array_element)))
      (Variables|/Game/RPGContent/Blueprints/SaveBP.SaveBP_C|SetTileProperties (Variables|Default|GetSaveRef) (LocalVariables|GetTempArray))
      (Variables|/Game/RPGContent/Blueprints/SaveBP.SaveBP_C|SetHexmapRadius (Variables|Default|GetSaveRef) (Variables|MapCreation|GetHexmapRadius))
      (Variables|/Game/RPGContent/Blueprints/SaveBP.SaveBP_C|SetSavename (Variables|Default|GetSaveRef) (Variables|MapCreation|GetSaveName))
      (Variables|/Game/RPGContent/Blueprints/SaveBP.SaveBP_C|SetPlayerTileIndex (Variables|Default|GetSaveRef) (Variables|MapCreation|GetPlayerTileIndex))
      (Variables|/Game/RPGContent/Blueprints/SaveBP.SaveBP_C|SetRandomSeed (Variables|Default|GetSaveRef) (Variables|MapCreation|GetRandomSeed)))
    (:then_1
      (bind _returnvalue_2 (SaveGame|SaveGametoSlot (Variables|Default|GetSaveRef) (Variables|MapCreation|GetSaveName)))
      (if _returnvalue_2
        (Development|PrintString (Utilities|String|Append (Variables|MapCreation|GetSaveName) " Map saved") true true "(R=0.000000,G=1.000000,B=0.000000,A=1.000000)")
        (else
          (Development|PrintString "Can't save map" true true "(R=1.000000,G=0.000000,B=0.000000,A=1.000000)"))))))

(fn LoadMap
  (Management|ForceDestroy)
  (bind _returnvalue (SaveGame|DoesSaveGameExist (Variables|MapCreation|GetSaveName)))
  (if _returnvalue
    (bind _returnvalue_2 (SaveGame|LoadGamefromSlot (Variables|MapCreation|GetSaveName)))
    (bind _assave_bp (Utilities|Casting|CastToSaveBP _returnvalue_2)
      (:then
        (Variables|Default|SetSaveRef _assave_bp)
        (Utilities|FlowControl|Sequence
          (:then_0
            ;[1 1 1] Load data
            (bind _output_get (Variables|MapCreation|SetHexmapRadius (Variables|/Game/RPGContent/Blueprints/SaveBP.SaveBP_C|GetHexmapRadius (Variables|Default|GetSaveRef))))
            (Variables|Default|SetHexDiameter (- (* _output_get 2) 1))
            (Variables|MapCreation|SetSaveName (Variables|/Game/RPGContent/Blueprints/SaveBP.SaveBP_C|GetSavename (Variables|Default|GetSaveRef)))
            (Variables|MapCreation|SetPlayerTileIndex (Variables|/Game/RPGContent/Blueprints/SaveBP.SaveBP_C|GetPlayerTileIndex (Variables|Default|GetSaveRef)))
            (bind _output_get_2 (Variables|MapCreation|SetRandomSeed (Variables|/Game/RPGContent/Blueprints/SaveBP.SaveBP_C|GetRandomSeed (Variables|Default|GetSaveRef))))
            (Math|Random|SetRandomStreamSeed (Variables|Default|GetRandomStream) _output_get_2))
          (:then_1
            (Development|PrintString (Utilities|String|Append (Variables|MapCreation|GetSaveName) " map loaded") true true "(R=0.000000,G=1.000000,B=0.000000,A=1.000000)")
            (Management|SpawnMap))))
      (:CastFailed
        (Development|PrintString "Can't load map" true true "(R=1.000000,G=0.000000,B=0.000000,A=1.000000)")))
    (else
      (Development|PrintString (Utilities|String|Append (Variables|MapCreation|GetSaveName) " Map doesn't exist") true true "(R=1.000000,G=0.000000,B=0.000000,A=1.000000)"))))

(fn Reload)

(fn TranslocateMap)

(fn SpawnMap
  (bind _hexdiameter (Variables|Default|GetHexDiameter))
  (bind _tilearray (Variables|Default|GetTileArray))
  (bind _returnvalue (- _hexdiameter 1))
  (for _index (range 0 _returnvalue)
    (for _index_2 (range 0 _returnvalue)
      (if (and (> _index_2 (- _index (Variables|MapCreation|GetHexmapRadius))) (<= _index_2 (+ _index (- (Variables|Default|GetHexDiameter) (Variables|MapCreation|GetHexmapRadius)))))
        (bind _returnvalue_2 (Game|SpawnActorfromClass "/Game/RPGContent/Blueprints/Tile.Tile_C" (Math|Transform|MakeTransform (Utilities|CalculateLocationfromHexCentre _index_2 _index) "0, 0, 0" "1,1,1") "Undefined" 0 false (Utilities|CoordstoIndex _index_2 _index) self (Utilities|Array|Get(acopy) (Variables|/Game/RPGContent/Blueprints/SaveBP.SaveBP_C|GetTileProperties (Variables|Default|GetSaveRef)) (Utilities|CoordstoIndex _index_2 _index)) 0))
        (Utilities|Array|Add _tilearray _returnvalue_2)
        (Variables|/Game/RPGContent/Blueprints/Tile.Tile_C|SetTileProperties _returnvalue_2 (Utilities|Array|Get(acopy) (Variables|/Game/RPGContent/Blueprints/SaveBP.SaveBP_C|GetTileProperties (Variables|Default|GetSaveRef)) (Utilities|CoordstoIndex _index_2 _index)))
        (else
          (Utilities|Array|Add _tilearray 0))))))

(fn CreateHexMap
  (bind _tilearray (Variables|Default|GetTileArray))
  (bind _hexdiameter (Variables|Default|GetHexDiameter))
  (bind _returnvalue (- _hexdiameter 1))
  (for _index (range 0 _returnvalue)
    (for _index_2 (range 0 _returnvalue)
      (if (and (> _index_2 (- _index (Variables|MapCreation|GetHexmapRadius))) (<= _index_2 (+ _index (- (Variables|Default|GetHexDiameter) (Variables|MapCreation|GetHexmapRadius)))))
        (bind _returnvalue_2 (Game|SpawnActorfromClass "/Game/RPGContent/Blueprints/Tile.Tile_C" (Math|Transform|MakeTransform (Utilities|CalculateLocationfromHexCentre _index_2 _index) "0, 0, 0" "1,1,1") "Undefined" 0 false (Utilities|CoordstoIndex _index_2 _index) self (Utilities|Struct|MakeTileProperties "NewEnumerator3" false (Utilities|Array|MakeArray "" "" "" "" "" "")) 0))
        (Utilities|Array|Add _tilearray _returnvalue_2)
        (else
          (Utilities|Array|Add _tilearray 0))))))

(fn ForceDestroy
  (bind _outactors (Actor|GetAllActorsOfClass "/Game/RPGContent/Blueprints/Tile.Tile_C"))
  (for _array_element _outactors
    (Actor|DestroyActor _array_element)
    (Utilities|Array|Clear (Variables|Default|GetTileArray))))

(fn GetNeighbours
  (params (Tile :type Tile%20Object%20Reference))
  (bind _index (Variables|/Game/RPGContent/Blueprints/Tile.Tile_C|GetIndex Tile))
  (bind (_row _column) (Utilities|IndextoCoords _index))
  (return (Utilities|Array|MakeArray (Utilities|Array|Get(acopy) (Variables|Default|GetTileArray) (Utilities|CoordstoIndex (+ _row 1) (+ _column 0))) (Utilities|Array|Get(acopy) (Variables|Default|GetTileArray) (Utilities|CoordstoIndex (+ _row 1) (+ _column 1))) (Utilities|Array|Get(acopy) (Variables|Default|GetTileArray) (Utilities|CoordstoIndex (+ _row 0) (+ _column 1))) (Utilities|Array|Get(acopy) (Variables|Default|GetTileArray) (Utilities|CoordstoIndex (+ _row -1) (+ _column 0))) (Utilities|Array|Get(acopy) (Variables|Default|GetTileArray) (Utilities|CoordstoIndex (+ _row -1) (+ _column -1))) (Utilities|Array|Get(acopy) (Variables|Default|GetTileArray) (Utilities|CoordstoIndex (+ _row 0) (+ _column -1))))))