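; Hex map tile that builds its appearance in the construction script from its TileProperties.
; Terrain type sets the mesh or material: highlands and mountains get index-based rotation and a decal, while water is lowered.
; Wooded tiles scatter mesh components using downward line traces at random points drawn from the hexmap's random stream.
; Borders flagged as roads get decals rotated in 60-degree steps around the center.
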(event EventBeginPlay)

(event Collision|EventActorBeginOverlap
  (params (OtherActor :type Actor%20Object%20Reference)))

(event EventTick
  (params (DeltaSeconds :type Float%20%28single-precision%29)))

(fn ConstructionScript
  (bind _returnvalue (Transformation|GetActorLocation))
  (bind _hextile_mesh (Variables|Default|GetHextile%20Mesh))
  (bind _defaultsceneroot (Variables|Default|GetDefaultSceneRoot))
  (bind _defaultsceneroot_2 (Variables|Default|GetDefaultSceneRoot))
  (bind _defaultsceneroot_3 (Variables|Default|GetDefaultSceneRoot))
  (bind _hexmapref (Variables|Default|GetHexmapRef))
  (bind _hextile_mesh_2 (Variables|Default|GetHextile%20Mesh))
  (bind _returnvalue_2 (Transformation|GetWorldRotation _defaultsceneroot))
  (bind _returnvalue_3 (Transformation|GetWorldRotation _defaultsceneroot_2))
  (bind _returnvalue_4 (Transformation|GetWorldLocation _defaultsceneroot_3))
  (bind _randomstream (Variables|/Game/RPGContent/Blueprints/Hexmap.Hexmap_C|GetRandomStream _hexmapref))
  (bind _returnvalue_5 (Math|Random|RandomUnitVectorinConeinDegreesfromStream (Math|Vector|MakeVector 0.0 0.0 1.0) 9e+01 _randomstream))
  (bind _returnvalue_6 (* _returnvalue_5 1.8e+02))
  (bind _returnvalue_7 (+ _returnvalue_4 _returnvalue_6))
  (Utilities|FlowControl|Sequence
    (:then_0
      (switch Utilities|FlowControl|Switch|SwitchonTerrainType (.terraintype (Variables|Default|GetTileProperties))
        (:NewEnumerator3
          ;[1 1 1] Grassland
          (if (Variables|Default|GetisSurface)
            (Components|StaticMesh|SetStaticMesh (Variables|Default|GetHextile%20Mesh) "/Game/RPGContent/Objects/hextile2Surface.hextile2Surface")))
        (:NewEnumerator2
          ;[1 1 1] Highlands
          (Components|StaticMesh|SetStaticMesh _hextile_mesh "/Game/RPGContent/Objects/HighlandsTile.HighlandsTile")
          (Transformation|SetWorldRotation _hextile_mesh (Math|Rotator|MakeRotator (.roll _returnvalue_2) (.pitch _returnvalue_2) (* (Variables|Default|GetIndex) 6e+01)) false false)
          (AddComponent|AddDecalComponent false (Math|Transform|MakeTransform "0.0,0.0,20.000000" (Math|Rotator|MakeRotator 0.0 0.0 (* (Variables|Default|GetIndex) 11.0)) "1.000000,1.000000,1.000000")))
        (:NewEnumerator1
          ;[1 1 1] Mountain
          (Components|StaticMesh|SetStaticMesh _hextile_mesh_2 "/Game/RPGContent/Objects/MountainTile.MountainTile")
          (Transformation|SetWorldRotation _hextile_mesh_2 (Math|Rotator|MakeRotator (.roll _returnvalue_3) (.pitch _returnvalue_3) (* (Variables|Default|GetIndex) 6e+01)) false false)
          (AddComponent|AddDecalComponent false (Math|Transform|MakeTransform "0.0,0.0,180.000000" (Math|Rotator|MakeRotator 0.0 0.0 (* (Variables|Default|GetIndex) 11.0)) "1.000000,1.000000,1.000000")))
        (:NewEnumerator0
          ;[1 1 1] Water
          (Rendering|Material|SetMaterial (Variables|Default|GetHextile%20Mesh) 0 "/Game/RPGContent/Materials/WaterLake.WaterLake")
          (Transformation|SetWorldLocation (Variables|Default|GetHextile%20Mesh) (Math|Vector|MakeVector (.x _returnvalue) (.y _returnvalue) (- (.z _returnvalue) 7e+01)) false false))))
    (:then_1
      ;[1 1 1] Wood
      (if (.iswood (Variables|Default|GetTileProperties))
        (for _index (range 1 50)
          (bind _outhit (Collision|LineTraceByChannel _returnvalue_7 (- _returnvalue_7 "0, 0,200.000000") "TraceTypeQuery1" true 0 "None" false "(R=1.000000,G=0.000000,B=0.000000,A=1.000000)" "(R=0.000000,G=1.000000,B=0.000000,A=1.000000)" 25.0))
          (AddComponent|AddStaticMeshComponent false (Math|Transform|MakeTransform (- (.Location (Collision|BreakHitResult _outhit)) _returnvalue_4) "0, 0, 0" "1.000000,1.000000,1.000000")))))
    (:then_2
      ;[1 1 1] Roads
      (for (_array_element _array_index) (.borderproperties (Variables|Default|GetTileProperties))
        (if (.isroad _array_element)
          (AddComponent|AddDecalComponent false (Math|Transform|MakeTransform (* (Math|Vector|RotateVector "0.000000,1.000000, 0" (* "0,-60.000000, 0" _array_index)) 108.0) (Math|Rotator|MakeRotator 0.0 9e+01 (+ (.Yaw (Math|Rotator|BreakRotator (* "0,-60.000000, 0" _array_index))) 9e+01)) "1.000000,1.000000,1.000000")))))))